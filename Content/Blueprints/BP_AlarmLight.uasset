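; BP_AlarmLight is a rotating alarm beacon actor that can be switched on and off.
; FSetAlarmActive stores the active flag and toggles visibility of two spotlights and a bulb, and BeginPlay calls it to start the light off.
; While active, Tick yaws the Pivot component at a constant, frame-rate-independent speed.
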(event EventBeginPlay
  (CallFunction|FSetAlarmActive false))

(event Collision|EventActorBeginOverlap
  (params (OtherActor :type Actor%20Object%20Reference)))

(event EventTick
  (params (DeltaSeconds :type Float%20%28single-precision%29))
  (if (Variables|Default|GetAlarmActive)
    (Transformation|AddLocalRotation (Variables|Default|GetPivot) (Math|Rotator|MakeRotator 0.0 0.0 (* DeltaSeconds 1.8e+02)) false false)))

(fn ConstructionScript)

(fn FSetAlarmActive
  (params (Active :type Boolean))
  (bind _output_get (Variables|Default|SetAlarmActive Active))
  (Rendering|SetVisibility (Variables|Default|GetSpotLight) _output_get false))