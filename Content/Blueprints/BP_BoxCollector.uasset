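; BP_BoxCollector is an interactable drop-off point that sorts delivered boxes by shape address, shown as a decal set in the construction script.
; On interact, it takes the player's item, compares addresses and negates points on a mismatch.
; Matching non-dangerous boxes get success SFX and VFX; mismatched or dangerous ones get failure feedback.
; It then briefly shows the points on a popup widget, moves the box and makes the player drop it.
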(event EventBeginPlay
  ;[0.15 0.15 0.15 0.5] Casta till WBPText
  (bind _aswbp_text_popup (Utilities|Casting|CastToWBP_TextPopup (UserInterface|GetWidget (Variables|Default|GetUIWidget))))
  (Variables|Default|Set%20 _aswbp_text_popup)
  ;[0.15 0.15 0.15 0.5] Ta bort default texten som syns
  (Default|SetText (Variables|Default|Get%20) " "))

(event EventTick
  (params (DeltaSeconds :type Float%20%28single-precision%29)))

(event EventOnInteract
  (params (InteractingPlayer :type Spm%20G5%20Character%20Object%20Reference))
  (bind _output_get (Variables|Default|SetItem (Class|SpmG5Character|GetItem InteractingPlayer)))
  (Class|BoxDestroyer|HandleBox _output_get InteractingPlayer))

(event EventHandleBox
  (params (Item :type Item%20Object%20Reference) (Player :type Spm%20G5%20Character%20Object%20Reference))
  (bind _vfxpoint (Variables|Default|GetVFXPoint))
  (bind _vfxpoint_2 (Variables|Default|GetVFXPoint))
  (bind _returnvalue (Transformation|GetWorldLocation _vfxpoint))
  (if (Utilities|IsValid Item)
    (Class|Item|SetHasBeenDroppedOff Item true)
    (Variables|Default|SetItem Item)
    (Variables|Default|SetPlayer Player)
    ;[0.15 0.15 0.15 0.5] Check Address
    (if (Utilities|Enum|Equal(Enum) (Class|Item|GetAddress (Variables|Default|GetItem)) (Variables|Default|GetAddress))
      (Variables|Default|SetCorrectAddresMultiplier 1)
      (if (Class|Item|GetIsDangerous (Variables|Default|GetItem))
        (Development|PrintString "INCORRECT sorting" :!label _label)
        (Class|FMODBlueprintStatics|PlayEventAttached "/Game/FMOD/Events/SFX/Box/SFX_BoxDeliver_No.SFX_BoxDeliver_No" _vfxpoint_2 "None" "0, 0, 0" "KeepRelativeOffset")
        (Niagara|SpawnSystematLocation "/Game/VFX/NS_WrongDelivery.NS_WrongDelivery" _returnvalue)
        (else
          (Development|PrintString "Correct sorting")
          (Class|FMODBlueprintStatics|PlayEventAttached "/Game/FMOD/Events/SFX/Box/SFX_BoxDeliver_Yes.SFX_BoxDeliver_Yes" _vfxpoint_2 "None" "0, 0, 0" "KeepRelativeOffset")
          (Niagara|SpawnSystematLocation "/Game/VFX/NS_SuccessfulDelivery.NS_SuccessfulDelivery" _returnvalue)))
      (else
        (Class|Item|SetNegativePoints (Variables|Default|GetItem))
        (Variables|Default|SetCorrectAddresMultiplier 1)
        (goto _label)))
    (Development|PrintString "SUCCESS")
    (Default|SetText (Variables|Default|Get%20) (Utilities|Text|ToText(Integer) (* (Variables|Default|GetCorrectAddresMultiplier) (Class|Item|GetPoints (Variables|Default|GetItem)))))
    (Transformation|SetActorLocation (Variables|Default|GetItem) (Transformation|GetWorldLocation (Variables|Default|GetWhereTheBoxGoes)) false false)
    (if (Utilities|IsValid (Variables|Default|GetPlayer))
      (Class|SpmG5Character|Drop (Variables|Default|GetPlayer)))
    (Utilities|FlowControl|Delay 1.5)
    (Default|SetText (Variables|Default|Get%20))))

(fn ConstructionScript
  (bind _address (Variables|Default|GetAddress))
  ;[0.15 0.15 0.15 0.5] Sätter vilken address den här ska ha samt sätter decal
  (Utilities|FlowControl|Sequence
    (:then_0
      (if (Utilities|Enum|Equal(Enum) _address "CIRCLE")
        (Rendering|Components|Decal|SetDecalMaterial (Variables|Default|GetAddressIcon) "/Game/UI/M_Decal_AddressCircle.M_Decal_AddressCircle")))
    (:then_1
      (if (Utilities|Enum|Equal(Enum) _address "SQUARE")
        (Rendering|Components|Decal|SetDecalMaterial (Variables|Default|GetAddressIcon) "/Game/UI/M_Decal_AddressSquare.M_Decal_AddressSquare")))
    (:then_2
      (if (Utilities|Enum|Equal(Enum) _address "TRIANGLE")
        (Rendering|Components|Decal|SetDecalMaterial (Variables|Default|GetAddressIcon) "/Game/UI/M_Decal_AddressTriangle.M_Decal_AddressTriangle")))))