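; Interactive radio actor that switches channels on interaction and reacts to the shift timer.
; On BeginPlay and each time change, it stores the remaining seconds and updates pitch, turning off when time runs out; the two bound handlers' names are swapped.
; Interaction plays a button sound, turns the radio off and deactivates NSRadioSound, then switches channel and reactivates it after a short delay.
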(event Custom|OnTimeChanged
  (Class|Radio|TurnOff))

(event Custom|OnTimeRunsOut
  (bind _returnvalue (Subsystems|GetShiftManager))
  (bind _returnvalue_2 (Class|ShiftManager|GetCurrentMin _returnvalue))
  (bind _returnvalue_3 (Class|ShiftManager|GetCurrentSec _returnvalue))
  (Variables|Default|SetTimeLeft (+ _returnvalue_3 (* _returnvalue_2 60)))
  (Class|Radio|UpdatePitch))

(event EventBeginPlay
  (bind _returnvalue (Subsystems|GetShiftManager))
  (bind _returnvalue_2 (Subsystems|GetShiftManager))
  (Utilities|FlowControl|Sequence
    (:then_0
      (EventDispatchers|BindEventtoOnTimeRunsOut _returnvalue_2 (delegate Custom|OnTimeChanged)))
    (:then_1
      (EventDispatchers|BindEventtoOnTimeChanged _returnvalue_2 (delegate Custom|OnTimeRunsOut)))
    (:then_2
      (bind _returnvalue_3 (Class|ShiftManager|GetCurrentMin _returnvalue))
      (bind _returnvalue_4 (Class|ShiftManager|GetCurrentSec _returnvalue))
      (Variables|Default|SetTimeLeft (+ _returnvalue_4 (* _returnvalue_3 60)))
      (Class|Radio|UpdatePitch))))

(event Collision|EventActorBeginOverlap
  (params (OtherActor :type Actor%20Object%20Reference)))

(event EventTick
  (params (DeltaSeconds :type Float%20%28single-precision%29)))

(event EventOnInteract
  (params (InteractingPlayer :type Spm%20G5%20Character%20Object%20Reference))
  (Development|PrintString "Switching Radio Channel")
  ;[0.15 0.15 0.15 0.5] RUBEN INSERT CLICK SOUND HERE
  (Class|FMODBlueprintStatics|PlayEventatLocation "/Game/FMOD/Events/SFX/Radio/SFX_RadioButton.SFX_RadioButton" (Transformation|GetActorTransform))
  (Class|Radio|TurnOff)
  (Components|Activation|Deactivate (Variables|Default|GetNS_RadioSound))
  (Utilities|FlowControl|Delay 0.7)
  (Class|Radio|SwitchChannel)
  (Components|Activation|Activate (Variables|Default|GetNS_RadioSound) false))

(fn ConstructionScript)