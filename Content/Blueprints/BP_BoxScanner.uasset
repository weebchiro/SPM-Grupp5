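; Scanner station that checks parcel Items and flags them as good or suspicious.
; Takes parcels through player interaction or throws landing high enough on an empty station; interacting when idle can also retrieve or swap the parcel.
; A Timeline sweeps the scanner over the attached parcel, then sets its scanned state and points.
; The result drives the parcel decal, UI icon, lamps and FMOD sound parameter.
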(event OnComponentHit(StaticMesh)
  (params (HitComponent :type Primitive%20Component%20Object%20Reference) (OtherActor :type Actor%20Object%20Reference) (OtherComp :type Primitive%20Component%20Object%20Reference) (NormalImpulse :type Vector :default "0, 0, 0") (Hit :type Hit%20Result%20Structure%20%28by%20ref%29))
  (bind _scanstart (Variables|Default|GetScanStart))
  (bind _relativelocation (Variables|/Script/Engine.SceneComponent|GetRelativeLocation _scanstart))
  (bind (_x _y _z) (Math|Vector|BreakVector _relativelocation))
  ;[0.15 0.15 0.15 0.5] Så man kan kasta in items i stationen!
  (bind _asitem (Utilities|Casting|CastToItem OtherActor))
  (bind _should_continue (CallFunction|HandleThrow _asitem))
  (if _should_continue
    (Variables|/Script/SpmG5.Item|SetbIsInStation (Variables|Default|GetScanningItem) true)
    (CallFunction|StartSFX)
    (Transformation|AttachComponentToComponent (Variables|Default|GetScanningItem) (Variables|Default|GetBoxHolder) "None" "SnapToTarget" "SnapToTarget" "KeepRelative" true)
    (Rendering|SetVisibility (Variables|Default|GetSM_ParcelScanner) true false)
    (Rendering|SetVisibility (Variables|Default|GetScanDecal) true false)
    (bind _duration (Timeline|Timeline PlayFromStart)
      (:Update
        (Class|MovieSceneTransformOrigin|GetTransformOrigin(Message) (Variables|Default|GetSM_ParcelScanner))
        (Transformation|SetRelativeLocation (Variables|Default|GetSM_ParcelScanner) (Math|Vector|MakeVector _x _y (Math|Float|Lerp _z (.Z (Math|Vector|BreakVector (Variables|/Script/Engine.SceneComponent|GetRelativeLocation (Variables|Default|GetScanBottom)))) _duration)) false false))
      (:Finished
        (Rendering|SetVisibility (Variables|Default|GetSM_ParcelScanner) false false)
        (Rendering|SetVisibility (Variables|Default|GetScanDecal) false false)
        (Variables|Default|SetisScanning false)
        (Utilities|IsValid (Variables|Default|GetScanningItem)
          (:Is%20Valid
            (Class|Item|SetIsScanned (Variables|Default|GetScanningItem) true)
            (Class|Item|SetPoints (Variables|Default|GetScanningItem))
            (if (Class|Item|GetIsSuspicious (Variables|Default|GetScanningItem))
              ;[0.15 0.15 0.15 0.5] visa ? dekal
              (Rendering|Components|Decal|SetDecalMaterial (Actor|GetComponentbyClass (Variables|Default|GetScanningItem) "/Script/Engine.DecalComponent") "/Game/UI/M_Decal_AddressQuestionmark.M_Decal_AddressQuestionmark")
              (Rendering|SetVisibility (Actor|GetComponentbyClass (Variables|Default|GetScanningItem) "/Script/Engine.DecalComponent") true false)
              (Development|PrintString "This package is SUS" true true "(R=1.000000,G=0.084021,B=0.000000,A=1.000000)")
              ;[0.15 0.15 0.15 0.5] Set SFX parameter - Ruben
              (Class|FMODAudioComponent|SetParameter (Variables|Default|GetFMOD%20SFX) "Success" 0.0)
              ;[0.15 0.15 0.15 0.5] Visar UI + lampor resultat
              (Rendering|Material|SetMaterial (Variables|Default|GetUIPlane) 0 "/Game/UI/M_IconQuestionmark.M_IconQuestionmark")
              (Rendering|SetVisibility (Variables|Default|GetParcelSus) true false)
              (else
                ;[0.15 0.15 0.15 0.5] visa dekal
                (Rendering|SetVisibility (Actor|GetComponentbyClass (Variables|Default|GetScanningItem) "/Script/Engine.DecalComponent") true false)
                (Development|PrintString "This package is GOOD" true true "(R=0.143894,G=1.000000,B=0.206475,A=1.000000)")
                (Class|FMODAudioComponent|SetParameter (Variables|Default|GetFMOD%20SFX) "Success" 1.0)
                (Rendering|Material|SetMaterial (Variables|Default|GetUIPlane) 0 "/Game/UI/M_IconCheckmark.M_IconCheckmark")
                (Rendering|SetVisibility (Variables|Default|GetParcelGood) true false)))
            (Rendering|SetVisibility (Variables|Default|GetUIPlane) true false)
            ;[0.15 0.15 0.15 0.5] Stop SFX and set it to null - Ruben
            (Class|FMODAudioComponent|Stop (Variables|Default|GetFMOD%20SFX))
            (Variables|Default|SetFMOD%20SFX 0)
            (Variables|Default|SetTempHeldItem 0))
          (:Is%20Not%20Valid
            (Variables|Default|SetScanningItem 0)))))))

(event EventOnInteract
  (params (InteractingPlayer :type Spm%20G5%20Character%20Object%20Reference))
  (bind _scanstart (Variables|Default|GetScanStart))
  (bind _relativelocation (Variables|/Script/Engine.SceneComponent|GetRelativeLocation _scanstart))
  (bind (_x _y _z) (Math|Vector|BreakVector _relativelocation))
  (Variables|Default|SetInteracting%20Player InteractingPlayer)
  (Utilities|IsValid (Variables|Default|GetScanningItem)
    (:Is%20Valid
      (if (Variables|Default|GetisScanning)
        (Development|PrintString "box is busy")
        ;[0.15 0.15 0.15 0.5] Visar UI resultat
        (Rendering|Material|SetMaterial (Variables|Default|GetUIPlane) 0 "/Game/UI/M_IconAlreadyFull.M_IconAlreadyFull")
        (Rendering|SetVisibility (Variables|Default|GetUIPlane) true false :!label _label)
        (Utilities|FlowControl|Delay 1.5)
        (Rendering|SetVisibility (Variables|Default|GetUIPlane) false false)
        (elif (Class|SpmG5Character|GetHasItem (Variables|Default|GetInteracting%20Player))
          (CallFunction|SwapBox)
          (Variables|/Script/SpmG5.Item|SetbIsInStation (Variables|Default|GetScanningItem) true :!label _label_2)
          (CallFunction|StartSFX)
          (Transformation|AttachComponentToComponent (Variables|Default|GetScanningItem) (Variables|Default|GetBoxHolder) "None" "SnapToTarget" "SnapToTarget" "KeepRelative" true)
          (Rendering|SetVisibility (Variables|Default|GetSM_ParcelScanner) true false)
          (Rendering|SetVisibility (Variables|Default|GetScanDecal) true false)
          (bind _duration (Timeline|Timeline PlayFromStart)
            (:Update
              (Class|MovieSceneTransformOrigin|GetTransformOrigin(Message) (Variables|Default|GetSM_ParcelScanner))
              (Transformation|SetRelativeLocation (Variables|Default|GetSM_ParcelScanner) (Math|Vector|MakeVector _x _y (Math|Float|Lerp _z (.Z (Math|Vector|BreakVector (Variables|/Script/Engine.SceneComponent|GetRelativeLocation (Variables|Default|GetScanBottom)))) _duration)) false false))
            (:Finished
              (Rendering|SetVisibility (Variables|Default|GetSM_ParcelScanner) false false)
              (Rendering|SetVisibility (Variables|Default|GetScanDecal) false false)
              (Variables|Default|SetisScanning false)
              (Utilities|IsValid (Variables|Default|GetScanningItem)
                (:Is%20Valid
                  (Class|Item|SetIsScanned (Variables|Default|GetScanningItem) true)
                  (Class|Item|SetPoints (Variables|Default|GetScanningItem))
                  (if (Class|Item|GetIsSuspicious (Variables|Default|GetScanningItem))
                    ;[0.15 0.15 0.15 0.5] visa ? dekal
                    (Rendering|Components|Decal|SetDecalMaterial (Actor|GetComponentbyClass (Variables|Default|GetScanningItem) "/Script/Engine.DecalComponent") "/Game/UI/M_Decal_AddressQuestionmark.M_Decal_AddressQuestionmark")
                    (Rendering|SetVisibility (Actor|GetComponentbyClass (Variables|Default|GetScanningItem) "/Script/Engine.DecalComponent") true false)
                    (Development|PrintString "This package is SUS" true true "(R=1.000000,G=0.084021,B=0.000000,A=1.000000)")
                    ;[0.15 0.15 0.15 0.5] Set SFX parameter - Ruben
                    (Class|FMODAudioComponent|SetParameter (Variables|Default|GetFMOD%20SFX) "Success" 0.0)
                    ;[0.15 0.15 0.15 0.5] Visar UI + lampor resultat
                    (Rendering|Material|SetMaterial (Variables|Default|GetUIPlane) 0 "/Game/UI/M_IconQuestionmark.M_IconQuestionmark")
                    (Rendering|SetVisibility (Variables|Default|GetParcelSus) true false)
                    (else
                      ;[0.15 0.15 0.15 0.5] visa dekal
                      (Rendering|SetVisibility (Actor|GetComponentbyClass (Variables|Default|GetScanningItem) "/Script/Engine.DecalComponent") true false)
                      (Development|PrintString "This package is GOOD" true true "(R=0.143894,G=1.000000,B=0.206475,A=1.000000)")
                      (Class|FMODAudioComponent|SetParameter (Variables|Default|GetFMOD%20SFX) "Success" 1.0)
                      (Rendering|Material|SetMaterial (Variables|Default|GetUIPlane) 0 "/Game/UI/M_IconCheckmark.M_IconCheckmark")
                      (Rendering|SetVisibility (Variables|Default|GetParcelGood) true false)))
                  (Rendering|SetVisibility (Variables|Default|GetUIPlane) true false)
                  ;[0.15 0.15 0.15 0.5] Stop SFX and set it to null - Ruben
                  (Class|FMODAudioComponent|Stop (Variables|Default|GetFMOD%20SFX))
                  (Variables|Default|SetFMOD%20SFX 0)
                  (Variables|Default|SetTempHeldItem 0))
                (:Is%20Not%20Valid
                  (Variables|Default|SetScanningItem 0)))))
          (else
            (CallFunction|PlayerPickup)))))
    (:Is%20Not%20Valid
      (if (Class|SpmG5Character|GetHasItem (Variables|Default|GetInteracting%20Player))
        (Variables|Default|SetisScanning true)
        (bind _returnvalue (Class|SpmG5Character|Drop (Variables|Default|GetInteracting%20Player)))
        (Variables|Default|SetScanningItem _returnvalue)
        (goto _label_2)
        (else
          (Development|PrintString "no box")
          (Rendering|Material|SetMaterial (Variables|Default|GetUIPlane) 0 "/Game/UI/M_IconNeedBox.M_IconNeedBox")
          (goto _label))))))

(fn ConstructionScript)

(fn StartSFX
  ;[0.15 0.15 0.15 0.5] Start SFX and stop if SFX already exists - Ruben
  (if (Utilities|IsValid (Variables|Default|GetFMOD%20SFX))
    (Class|FMODAudioComponent|Stop (Variables|Default|GetFMOD%20SFX)))
  (bind _returnvalue (Class|FMODBlueprintStatics|PlayEventAttached "/Game/FMOD/Events/SFX/Stations/SFX_Scanner.SFX_Scanner" (Variables|Default|GetBoxHolder) "None" "0, 0, 0" "KeepRelativeOffset"))
  (Variables|Default|SetFMOD%20SFX _returnvalue))

(fn PlayerPickup
  (Transformation|DetachFromActor (Variables|Default|GetScanningItem) "KeepWorld" "KeepWorld" "KeepWorld")
  (Class|SpmG5Character|Pickup (Variables|Default|GetInteracting%20Player) (Variables|Default|GetScanningItem))
  (Variables|/Script/SpmG5.Item|SetbIsInStation (Variables|Default|GetScanningItem) false)
  (Variables|Default|SetScanningItem 0)
  (Variables|Default|SetInteracting%20Player 0)
  ;[0.15 0.15 0.15 0.5] Gör UI + lampor invis
  (Rendering|SetVisibility (Variables|Default|GetUIPlane) false false)
  (Rendering|SetVisibility (Variables|Default|GetParcelGood) false false)
  (Rendering|SetVisibility (Variables|Default|GetParcelSus) false false))

(fn SwapBox
  (Variables|Default|SetTempHeldItem (Variables|/Script/SpmG5.SpmG5Character|GetHeldItem (Variables|Default|GetInteracting%20Player)))
  (Class|SpmG5Character|Drop (Variables|Default|GetInteracting%20Player))
  (Utilities|FlowControl|Sequence
    (:then_0
      (Niagara|SpawnSystematLocation "/Game/VFX/NS_SwitchPacketSmoke.NS_SwitchPacketSmoke" (Transformation|GetWorldLocation (Variables|Default|GetBoxHolder)) "0, 0, 0" "1.000000,1.000000,2.000000")
      (Niagara|SpawnSystematLocation "/Game/VFX/NS_SwitchPacketSmoke.NS_SwitchPacketSmoke" (Transformation|GetActorLocation (Variables|Default|GetTempHeldItem)) "0, 0, 0" "1.000000,1.000000,2.000000"))
    (:then_1
      (Utilities|FlowControl|Sequence
        (:then_0
          (CallFunction|PlayerPickup))
        (:then_1
          (Variables|Default|SetScanningItem (Variables|Default|GetTempHeldItem))
          (Variables|Default|SetisScanning true))))))

(fn HandleThrow
  (params (Item :type Item%20Object%20Reference))
  (if (>= (.Z (Math|Vector|BreakVector (Transformation|GetActorLocation Item))) (+ (.Z (Math|Vector|BreakVector (Transformation|GetActorLocation))) 5e+01))
    (Utilities|IsValid (Variables|Default|GetScanningItem)
      (:Is%20Not%20Valid
        (Development|PrintString "Should interact with item!!")
        (Variables|Default|SetisScanning true)
        (Variables|Default|SetScanningItem Item)
        (return true)))
    (else
      (return false))))