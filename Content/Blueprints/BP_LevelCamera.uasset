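; Shared level camera for two players that becomes the view target and anchors both controllers' audio listeners to itself.
; While GameManager allows movement in a level, Tick eases it toward the players' midpoint, clamped around its construction-time position at fixed height.
; FOV eases wider when either player is far from that start position or close on X, then narrows back.
; Idle shake and look-at rotation are disconnected, noted as causing motion sickness.
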(event EventBeginPlay
  (Game|Player|SetViewTargetwithBlend (Game|GetPlayerController 0) self 0.0 "VTBlend_Linear" 0.0 false)
  (if (Variables|/Game/BP_GameManager.BP_GameManager_C|GetShouldCameraMove (CallFunction|GetGameManager))
    _))

(event EventTick
  (params (DeltaSeconds :type Float%20%28single-precision%29))
  (Class|PlayerController|SetAudioListenerOverride (Game|GetPlayerController 0) (Variables|CameraActor|GetCameraComponent) "0, 0, 0" "0, 0, 0")
  (Class|PlayerController|SetAudioListenerOverride (Game|GetPlayerController 1) (Variables|CameraActor|GetCameraComponent) "0, 0, 0" "0, 0, 0")
  (if (Variables|/Game/BP_GameManager.BP_GameManager_C|GetShouldCameraMove (CallFunction|GetGameManager))
    ;[0.15 0.15 0.15 0.5] Only move camera while in level
    (if (Variables|/Game/BP_GameManager.BP_GameManager_C|GetbIsInLevel (CallFunction|GetGameManager))
      (CallFunction|ChangeFOV DeltaSeconds)
      (CallFunction|MovetoPlayers DeltaSeconds))))

(fn ConstructionScript
  (Variables|Default|SetCameraStartPos (Transformation|GetActorLocation)))

(fn ChangeFOV
  (params (Time :type Float%20%28double-precision%29))
  (bind _returnvalue (* Time 0.1))
  (bind _bisplayerfarfromcamera (CallFunction|IsPlayerFarfromCamera))
  (bind _bisplayerclosetocamera (CallFunction|IsPlayerClosetoCamera))
  (if (or _bisplayerfarfromcamera _bisplayerclosetocamera)
    ;[0.15 0.15 0.15 0.5] Increase FOV
    (Camera|SetFieldOfView (Variables|CameraActor|GetCameraComponent) (Math|Float|Lerp (Variables|/Script/Engine.CameraComponent|GetFieldOfView (Variables|CameraActor|GetCameraComponent)) (Variables|Default|GetMaxFOV) (* Time 0.1)))
    (Variables|Default|SetbIsFOVIncreased true)
    (elif (Variables|Default|GetbIsFOVIncreased)
      ;[0.15 0.15 0.15 0.5] Decrease FOV
      (Camera|SetFieldOfView (Variables|CameraActor|GetCameraComponent) (Math|Float|Lerp (Variables|/Script/Engine.CameraComponent|GetFieldOfView (Variables|CameraActor|GetCameraComponent)) (Variables|Default|GetMinFOV) _returnvalue))
      (if (>= _returnvalue 1.0)
        (Variables|Default|SetbIsFOVIncreased false)))))

(fn ChangeRotation
  (params (Time :type Float%20%28double-precision%29))
  (bind _cameracomponent (Variables|CameraActor|GetCameraComponent))
  ;[0.15 0.15 0.15 0.5] ADJUST CAMERA ROTATION AROUND PLAYERS MIDPOINT
  (bind _point (CallFunction|FindPointBetweenPlayers))
  (Transformation|SetWorldRotation _cameracomponent (Math|Rotator|Lerp(Rotator) (Transformation|GetWorldRotation _cameracomponent) (Math|Rotator|MakeRotator (.roll (Math|Rotator|FindLookatRotation (Transformation|GetWorldLocation (Variables|CameraActor|GetCameraComponent)) _point)) (Math|Float|ClampAngle (.pitch (Math|Rotator|FindLookatRotation (Transformation|GetWorldLocation (Variables|CameraActor|GetCameraComponent)) _point)) -58.0 -52.0) (.yaw (Transformation|GetWorldRotation (Variables|CameraActor|GetCameraComponent)))) (* Time 0.09)) false false))

(fn MovetoPlayers
  (params (Time :type Float%20%28double-precision%29))
  (bind _camerastartpos (Variables|Default|GetCameraStartPos))
  (bind _maxposxdiff (Variables|Default|GetMaxPosXDiff))
  (bind _camerastartpos_2 (Variables|Default|GetCameraStartPos))
  (bind _maxposydiff (Variables|Default|GetMaxPosYDiff))
  (bind _point (CallFunction|FindPointBetweenPlayers))
  (Transformation|SetActorLocation (Math|Vector|Lerp(Vector) (Transformation|GetActorLocation) (Math|Vector|MakeVector (Math|Float|Clamp(Float) (.x _point) (- (.x _camerastartpos_2) _maxposxdiff) (+ (.x _camerastartpos_2) _maxposxdiff)) (Math|Float|Clamp(Float) (.y _point) (- (.y _camerastartpos) _maxposydiff) (+ (.y _camerastartpos) _maxposydiff)) (.z (Variables|Default|GetCameraStartPos))) (* Time 0.2)) false false))

(fn FindPointBetweenPlayers
  (bind _returnvalue (Game|Player|GetPlayerPawn 1))
  (bind _returnvalue_2 (Transformation|GetActorLocation _returnvalue))
  (return (+ (/ (- (Transformation|GetActorLocation (Game|Player|GetPlayerPawn 0)) _returnvalue_2) 2) _returnvalue_2)))

(fn IsPlayerFarfromCamera
  (return (or (or (> (Math|Float|Absolute(Float) (- (.x (Transformation|GetActorLocation (Game|Player|GetPlayerPawn 0))) (.x (Variables|Default|GetCameraStartPos)))) (Variables|Default|GetXFarDistToCameraLedge_0)) (> (Math|Float|Absolute(Float) (- (.y (Transformation|GetActorLocation (Game|Player|GetPlayerPawn 0))) (.y (Variables|Default|GetCameraStartPos)))) (Variables|Default|GetYFarDistToCameraLedge))) (or (> (Math|Float|Absolute(Float) (- (.x (Transformation|GetActorLocation (Game|Player|GetPlayerPawn 1))) (.x (Variables|Default|GetCameraStartPos)))) (Variables|Default|GetXFarDistToCameraLedge_0)) (> (Math|Float|Absolute(Float) (- (.y (Transformation|GetActorLocation (Game|Player|GetPlayerPawn 1))) (.y (Variables|Default|GetCameraStartPos)))) (Variables|Default|GetYFarDistToCameraLedge))))))

(fn IsPlayerClosetoCamera
  (return (or (< (Math|Float|Absolute(Float) (- (.x (Transformation|GetActorLocation (Game|Player|GetPlayerPawn 0))) (.x (Variables|Default|GetCameraStartPos)))) (Variables|Default|GetXCloseDistToCameraLedge)) (< (Math|Float|Absolute(Float) (- (.x (Transformation|GetActorLocation (Game|Player|GetPlayerPawn 1))) (.x (Variables|Default|GetCameraStartPos)))) (Variables|Default|GetXCloseDistToCameraLedge)))))