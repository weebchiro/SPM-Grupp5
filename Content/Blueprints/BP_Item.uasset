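; BP_Item is a throwable parcel with an address, fragile and large variants, and an outline overlay highlight.
; Construction picks the box mesh, sets address and fragile decals (address icon starts hidden), and feeds color and surface values into dynamic materials.
; Hits above a speed threshold spawn impact VFX and optional sound, gated by a cooldown.
; A looping timer toggles the throw trail by speed, starting it only after someone has held the parcel.
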(event OnComponentHit(BaseMesh)
  (params (HitComponent :type Primitive%20Component%20Object%20Reference) (OtherActor :type Actor%20Object%20Reference) (OtherComp :type Primitive%20Component%20Object%20Reference) (NormalImpulse :type Vector :default "0, 0, 0") (Hit :type Hit%20Result%20Structure%20%28by%20ref%29))
  (bind (_bblockinghit _binitialoverlap _time _distance _location _impactpoint _normal _impactnormal) (Collision|BreakHitResult Hit))
  ;[0.15 0.15 0.15 0.5] Impact VFX
  (if (and (Variables|Default|GetCanPlayImpact) (> (Math|Vector|VectorLength (Transformation|GetComponentVelocity (Variables|Default|GetBaseMesh))) (Variables|Default|GetImpactThreshold)))
    (Niagara|SpawnSystematLocation "/Game/VFX/NS_ParcelImpact.NS_ParcelImpact" (+ _impactpoint (* _impactnormal (Variables|Default|GetImpactOffsetMult))) (Math|Rotator|MakeRotfromZ _impactnormal))
    (if (Variables|Default|GetPlaySound)
      (Class|FMODBlueprintStatics|PlayEventAttached "/Game/FMOD/Events/SFX/Box/SFX_BoxCartoonImpact.SFX_BoxCartoonImpact" (Variables|Default|GetBaseMesh) "None" "0, 0, 0" "KeepRelativeOffset" true))
    (Variables|Default|SetCanPlayImpact false)
    (Utilities|FlowControl|Delay 0.5)
    (Variables|Default|SetCanPlayImpact true)))

(event Custom|Set%20Values
  (for _array_element (Variables|Default|GetDynamicMaterials)
    (Rendering|Material|SetVectorParameterValue _array_element "Color" (Variables|Default|GetColor) :!class /Script/Engine.MaterialInstanceDynamic)
    (Rendering|Material|SetScalarParameterValue _array_element "Roughness" (Variables|Default|GetRoughness) :!class /Script/Engine.MaterialInstanceDynamic)
    (Rendering|Material|SetScalarParameterValue _array_element "Metallic" (Variables|Default|GetMetallic) :!class /Script/Engine.MaterialInstanceDynamic)
    (Rendering|Material|SetScalarParameterValue _array_element "Emission" (Variables|Default|GetEmission) :!class /Script/Engine.MaterialInstanceDynamic)))

(event Custom|UpdateItemTrail
  ;[0.15 0.15 0.15 0.5] Throw Trail VFX
  (Utilities|FlowControl|Sequence
    (:then_0
      (if (and (Utilities|IsValid (Variables|Default|GetMostRecentHolder)) (and (> (Math|Vector|VectorLength (Transformation|GetComponentVelocity (Variables|Default|GetBaseMesh))) (Variables|Default|GetTrailSpeedThreshold)) (not (Variables|Default|GetTrailActive))))
        (Variables|Default|SetTrailActive true)
        (Components|Activation|Activate (Variables|Default|GetThrowTrailVFX) false)))
    (:then_1
      (if (and (< (Math|Vector|VectorLength (Transformation|GetComponentVelocity (Variables|Default|GetBaseMesh))) (Variables|Default|GetTrailStopThreshold)) (Variables|Default|GetTrailActive))
        (Variables|Default|SetTrailActive false)
        (Components|Activation|Deactivate (Variables|Default|GetThrowTrailVFX))))))

(event EventBeginPlay
  (Utilities|FlowControl|Sequence
    (:then_0
      ;[0.15 0.15 0.15 0.5] Throw Trail VFX
      (Utilities|Time|SetTimerbyEvent (delegate Custom|UpdateItemTrail) 0.05 true))
    (:then_1
      (Utilities|FlowControl|Delay 1.0)
      (Variables|Default|SetCanPlayImpact true))))

(event EventSetAddressDecal
  (CallFunction|DoSetAddressDecal))

(fn ConstructionScript
  (bind _basemesh (Variables|Default|GetBaseMesh))
  (bind _basemesh_2 (Variables|Default|GetBaseMesh))
  (CallFunction|DoSetAddressDecal)
  (Rendering|SetVisibility (Variables|Default|GetAddressIcon) false false)
  ;[0.15 0.15 0.15 0.5] Creates a dynamic material
  (for (_array_element _array_index) (Rendering|Material|GetMaterials _basemesh_2)
    (bind _returnvalue (Rendering|Material|CreateDynamicMaterialInstance _basemesh_2 _array_index _array_element "None" :!class /Script/Engine.PrimitiveComponent))
    (Rendering|Material|SetMaterial (Variables|Default|GetBaseMesh) _array_index _returnvalue)
    (Utilities|Array|Add (Variables|Default|GetDynamicMaterials) _returnvalue))
  (Utilities|FlowControl|Sequence
    (:then_0
      ;[0.15 0.15 0.15 0.5] Set material if fragile
      (if (Class|Item|GetIsFragile)
        (Rendering|SetVisibility (Variables|Default|GetFragileDecal) true false)
        (else
          (Variables|Default|SetColor "(R=1.000000,G=0.431134,B=0.091144,A=1.000000)"))))
    (:then_1
      ;[0.15 0.15 0.15 0.5] Set Material if large box
      (if (Class|Item|GetIsLarge)
        (Components|StaticMesh|SetStaticMesh _basemesh "/Game/LevelPrototyping/Meshes/SM_Box_Big.SM_Box_Big")
        (else
          (Components|StaticMesh|SetStaticMesh _basemesh "/Game/LevelPrototyping/Meshes/SM_Box_Small.SM_Box_Small"))))
    (:then_2
      ;[0.15 0.15 0.15 0.5] Set material if dangerous
      (if (Class|Item|GetIsSuspicious)
        _))
    (:then_3
      (CallFunction|SetValues))))

(fn DoSetAddressDecal
  (bind _returnvalue (Class|Item|GetAddress))
  ;[0.15 0.15 0.15 0.5] Sätter vilken address den här ska ha samt sätter decal
  (Utilities|FlowControl|Sequence
    (:then_0
      (if (Utilities|Enum|Equal(Enum) _returnvalue "CIRCLE")
        (Rendering|Components|Decal|SetDecalMaterial (Variables|Default|GetAddressIcon) "/Game/UI/M_Decal_AddressCircle.M_Decal_AddressCircle")))
    (:then_1
      (if (Utilities|Enum|Equal(Enum) _returnvalue "SQUARE")
        (Rendering|Components|Decal|SetDecalMaterial (Variables|Default|GetAddressIcon) "/Game/UI/M_Decal_AddressSquare.M_Decal_AddressSquare")))
    (:then_2
      (if (Utilities|Enum|Equal(Enum) _returnvalue "TRIANGLE")
        (Rendering|Components|Decal|SetDecalMaterial (Variables|Default|GetAddressIcon) "/Game/UI/M_Decal_AddressTriangle.M_Decal_AddressTriangle")))))

(fn ActivateOvelay
  (params (SetTo :type Boolean))
  (if SetTo
    ;[0.15 0.15 0.15 0.5] Viktors (better) way of higligt
    (Rendering|Material|SetOverlayMaterial (Variables|Default|GetBaseMesh) "/Game/Materials/M_Outline1_Inst.M_Outline1_Inst" :!class /Script/Engine.MeshComponent)
    (else
      (Rendering|Material|SetOverlayMaterial (Variables|Default|GetBaseMesh) 0 :!class /Script/Engine.MeshComponent)))
  (return))