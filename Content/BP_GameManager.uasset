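; BP_GameManager is the central game manager that creates the UI widgets and drives level loading, menu return, pausing and saving.
; LoadLevel configures the AI spawner and shift timer from the current level info, stops menu music, then async-loads the level, with HUD and countdown skipped for tutorials.
; LoadMenu saves scores, restores menu UI and music, and resets the player character.
; Save stores high scores alongside settings, while pausing toggles the pause widget, cursor and input mode.
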(event Custom|Save
  (bind _output_get (Variables|Default|SetSaveState (Utilities|Struct|MakeGameData (Variables|/Script/SpmG5.ScoreManager|GetScoreMap (Subsystems|GetScoreManager)) (.MasterVolume (Utilities|Struct|BreakGameData (Variables|Default|GetSaveState))) (.MusicVolume (Utilities|Struct|BreakGameData (Variables|Default|GetSaveState))) (.SFXVolume (Utilities|Struct|BreakGameData (Variables|Default|GetSaveState))) (.StopCameraMove (Utilities|Struct|BreakGameData (Variables|Default|GetSaveState))))))
  (Class|SaveManager|SaveGame _output_get))

(event Custom|Load
  (Class|SaveManager|LoadGame)
  (Development|PrintString "mi bumclart"))

(event Custom|LoadMenu
  (bind _customcontroller1 (CallFunction|GetGameController))
  (bind _menu (Variables|Default|GetMenu))
  ;[0.15 0.15 0.15 0.5] Loads menu
  (Variables|Default|SetCanPause false)
  (Class|ScoreManager|SaveScore (Subsystems|GetScoreManager))
  (Default|UpdateHighscoreUI _menu)
  (UserInterface|Viewport|AddtoViewport _menu 0)
  (Variables|Default|SetbIsInLevel false)
  (|LoadLevelAsync "/Game/Levels/Menu.Menu"
    (:then
      (Widget|RemovefromParent (Variables|Default|GetHud)))
    (:OnLevelLoaded
      (Development|PrintString "cooked")
      (Variables|/Script/Engine.PlayerController|SetbShowMouseCursor _customcontroller1 true)
      (Input|SetInputModeUIOnly _customcontroller1 (Variables|Default|GetMenu) "DoNotLock" false)
      (bind _returnvalue (Class|FMODBlueprintStatics|PlayEvent2D "/Game/FMOD/Events/Music/Mu_MainMenu.Mu_MainMenu"))
      (Variables|Default|SetMusicInstance _returnvalue)
      (Default|ResetCharacter (.Player%20Character%201 (CallFunction|GetPlayerCharacter))))))

(event Custom|Load%20Level
  (bind _customcontroller1 (CallFunction|GetGameController))
  (bind _musicinstance (Variables|Default|GetMusicInstance))
  (bind _hud (Variables|Default|GetHud))
  (bind _currentlevelinfo (Variables|Default|GetCurrentLevelInfo))
  (bind _currentlevelinfo_2 (Variables|Default|GetCurrentLevelInfo))
  (bind (_level _pointstopass _shifttime _levelname _istutorial _amountofboxesperlevel _spawnrates _dangeroustypes _boxaddresses) (Utilities|Struct|BreakLevelInfo _currentlevelinfo))
  (bind (_level_2 _pointstopass_2 _shifttime_2 _levelname_2 _istutorial_2) (Utilities|Struct|BreakLevelInfo _currentlevelinfo_2))
  (Class|SpawnAI|SetupSpawner (Subsystems|GetSpawnAI) _amountofboxesperlevel _spawnrates _dangeroustypes _boxaddresses)
  ;[0.15 0.15 0.15 0.5] Loads level from level button
  (Class|ShiftManager|SetShiftTime (Subsystems|GetShiftManager) (.ShiftTime (Utilities|Struct|BreakLevelInfo (Variables|Default|GetCurrentLevelInfo))))
  (bind _returnvalue (Class|FMODBlueprintStatics|EventInstanceIsValid _musicinstance))
  (if _returnvalue
    (Class|FMODBlueprintStatics|EventInstanceStop _musicinstance false))
  (if (.IsTutorial (Utilities|Struct|BreakLevelInfo (Variables|Default|GetCurrentLevelInfo)))
    _
    (else
      (if (UserInterface|Viewport|IsinViewport (Variables|Default|GetHud))
        (Widget|RemovefromParent (Variables|Default|GetHud)))
      (UserInterface|Viewport|AddtoViewport _hud 0)
      (Default|SetStartTime _hud (.ShiftTime (Utilities|Struct|BreakLevelInfo (Variables|Default|GetCurrentLevelInfo))))
      (Class|ShiftManager|StartTimer (Subsystems|GetShiftManager))))
  (|LoadLevelAsync _level_2
    (:then
      (Widget|RemovefromParent (Variables|Default|GetMenu))
      (Widget|RemovefromParent (Variables|Default|GetInstructionWidget)))
    (:OnLevelLoaded
      (Utilities|FlowControl|Delay 0.1)
      (if _istutorial_2
        _
        (else
          (UserInterface|Viewport|AddtoViewport (Variables|Default|GetStartCountdown) 0)
          (Default|PlayCountdown (Variables|Default|GetStartCountdown))))
      (Variables|/Script/Engine.PlayerController|SetbShowMouseCursor _customcontroller1 false)
      (Variables|Default|SetbIsInLevel true)
      (Input|SetInputModeGameOnly _customcontroller1 false))))

(event EventPauseGame
  (CallFunction|Pause))

(event EventInit
  ;[0.15 0.15 0.15 0.5] Loads all necessary widgets
  (Utilities|FlowControl|Sequence
    (:then_0
      (bind _returnvalue (UserInterface|CreateWidget "/Game/Widgets/WBP_HUD.WBP_HUD_C"))
      (Variables|Default|SetHud _returnvalue)
      (bind _returnvalue_2 (UserInterface|CreateWidget "/Game/Widgets/WBP_Menu.WBP_Menu_C"))
      (Variables|Default|SetMenu _returnvalue_2)
      (bind _returnvalue_3 (UserInterface|CreateWidget "/Game/Widgets/WBP_InstructionFlowChart.WBP_InstructionFlowChart_C"))
      (Variables|Default|SetInstructionWidget _returnvalue_3)
      (bind _returnvalue_4 (UserInterface|CreateWidget "/Game/Widgets/WBP_ControllerMap.WBP_ControllerMap_C"))
      (Variables|Default|SetControllerWidget _returnvalue_4))
    (:then_1
      (bind _returnvalue_5 (UserInterface|CreateWidget "/Game/Widgets/WBP_WinOrLoseScreen.WBP_WinOrLoseScreen_C"))
      (Variables|Default|SetWinOrLoseWidget _returnvalue_5)
      (bind _returnvalue_6 (UserInterface|CreateWidget "/Game/Widgets/WBP_Pause.WBP_Pause_C"))
      (Variables|Default|SetPauseWidget _returnvalue_6)
      (bind _returnvalue_7 (UserInterface|CreateWidget "/Game/Widgets/WBP_Settings.WBP_Settings_C"))
      (Variables|Default|SetSettingsWidget _returnvalue_7))
    (:then_2
      (bind _returnvalue_8 (UserInterface|CreateWidget "/Game/Widgets/WBP_StartLevelCountdown.WBP_StartLevelCountdown_C"))
      (Variables|Default|SetStartCountdown _returnvalue_8)
      (bind _returnvalue_9 (UserInterface|CreateWidget "/Game/Widgets/WBP_ResultScreen.WBP_ResultScreen_C"))
      (Variables|Default|SetResultsWidget _returnvalue_9))
    (:then_3
      (EventDispatchers|BindEventtoLoadDispatcher (delegate Custom|Load)))))

(fn Pause
  (bind _customcontroller1 (CallFunction|GetGameController))
  (bind _pausewidget (Variables|Default|GetPauseWidget))
  (if (Variables|Default|GetCanPause)
    (Game|SetGamePaused (Class|KismetMathLibrary|XORBoolean (Game|IsGamePaused) true))
    (if (Game|IsGamePaused)
      (UserInterface|Viewport|AddtoViewport _pausewidget 0)
      (Input|SetInputModeGameandUI _customcontroller1 0 "DoNotLock" true false)
      (else
        (Widget|RemovefromParent _pausewidget)
        (Input|SetInputModeGameOnly _customcontroller1 false)))
    (Variables|/Script/Engine.PlayerController|SetbShowMouseCursor (.CustomController1 (CallFunction|GetGameController)) (Game|IsGamePaused))))